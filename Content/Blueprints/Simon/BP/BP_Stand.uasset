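; BP_Stand is an interactable colored pad in a Simon memory game, identified by an index and lit through a dynamic material instance.
; On interact by a player during the player's turn, it reports its index to the Simon main reference.
; PlayNote flashes its emissive intensity for a second, and PlayError flashes red before restoring its color.
; Looking at it during that turn shows a highlight overlay, cleared by a short retriggerable delay once the gaze leaves.
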(event `/Game/Blueprints/Simon/BP/BPI_Interface.OnInteract`
  (params (Actor :type "Actor Object Reference"))
  (if (`KismetSystemLibrary.DoesImplementInterface` Actor "/Game/Blueprints/Simon/BP/BPI_Player.BPI_Player_C")
    (bind _simonmainref (`self.SimonMainRef`)
      (:`then`
        (if (`/Game/Blueprints/Simon/BP/BP_Simon.IsPlayerTurn` _simonmainref)
          (`/Game/Blueprints/Simon/BP/BP_Simon.PlayerPlayedNote` (`self.SimonMainRef`) (`self.Index`))))
      (:`else`))))

(event `PlayNote`
  (`MaterialInstanceDynamic.SetScalarParameterValue` (`self.DynMat`) "Intensity" 8.0)
  (`KismetSystemLibrary.Delay` 1.0)
  (`MaterialInstanceDynamic.SetScalarParameterValue` (`self.DynMat`) "Intensity" 0.0))

(event `/Game/Blueprints/Simon/BP/BPI_Interface.OnLookAt`
  (params (Actor :type "Actor Object Reference"))
  (bind _simonmainref (`self.SimonMainRef`)
    (:`then`
      (if (`/Game/Blueprints/Simon/BP/BP_Simon.IsPlayerTurn` _simonmainref)
        (`MeshComponent.SetOverlayMaterial` (`self.Capsule`) "/Game/Blueprints/Simon/Mat/M_Overlay.M_Overlay")
        (`KismetSystemLibrary.RetriggerableDelay` 0.11)
        (`MeshComponent.SetOverlayMaterial` (`self.Capsule`) null)))
    (:`else`)))

(event `PlayError`
  (`MaterialInstanceDynamic.SetVectorParameterValue` (`self.DynMat`) "Color" (struct :`R` 1.0 :`A` 1.0))
  (`MaterialInstanceDynamic.SetScalarParameterValue` (`self.DynMat`) "Intensity" 8.0)
  (`KismetSystemLibrary.Delay` 1.0)
  (`MaterialInstanceDynamic.SetScalarParameterValue` (`self.DynMat`) "Intensity" 0.0)
  (`MaterialInstanceDynamic.SetVectorParameterValue` (`self.DynMat`) "Color" (`self.Color`)))

(fn `UserConstructionScript`
  (bind _returnvalue (`PrimitiveComponent.CreateDynamicMaterialInstance` (`self.Capsule`) 0 "/Game/Blueprints/Simon/Mat/M_Color.M_Color" "None"))
  (bind _output_get (set `self.DynMat` _returnvalue))
  (`MaterialInstanceDynamic.SetVectorParameterValue` _output_get "Color" (`self.Color`)))